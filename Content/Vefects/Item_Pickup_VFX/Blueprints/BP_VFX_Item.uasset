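; BP_VFX_Item is an item pickup VFX actor that gets launched and plays an aura effect where it hits.
; SetItemVFX assigns the aura, trail and sound assets, then turns on physics and launches the collision component in a fixed forward-and-upward arc.
; Tick keeps the collision unrotated, and a hit stops physics and activates the aura after a short delay.
; A timeline for scaling the aura exists but is never triggered.
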(event OnComponentHit(Collision)
  (params (HitComponent :type Primitive%20Component%20Object%20Reference) (OtherActor :type Actor%20Object%20Reference) (OtherComp :type Primitive%20Component%20Object%20Reference) (NormalImpulse :type Vector :default "0, 0, 0") (Hit :type Hit%20Result%20Structure%20%28by%20ref%29))
  (Physics|SetSimulatePhysics (Variables|Default|GetCollision) false)
  (Utilities|FlowControl|Delay 0.05)
  (Components|Activation|Activate (Variables|Default|GetItemAura) false))

(event Custom|Set%20Item%20VFX
  (params (VFX :type Niagara%20System%20Object%20Reference) (Trail :type Niagara%20System%20Object%20Reference) (SFX :type Sound%20Base%20Object%20Reference))
  (bind _collision (Variables|Default|GetCollision))
  ;[0.7478 1 0.2155] Set up Item
  (Class|NiagaraComponent|SetAsset (Variables|Default|GetItemAura) VFX true)
  (Class|NiagaraComponent|SetAsset (Variables|Default|GetTrailVFX) Trail true)
  (Audio|Components|Audio|SetSound (Variables|Default|GetAudio) SFX)
  (Physics|SetSimulatePhysics _collision true)
  (Class|PrimitiveComponent|SetAllPhysicsLinearVelocity _collision "700.000000, 0,500.000000" false))

(event EventTick
  (params (DeltaSeconds :type Float%20%28single-precision%29))
  (Transformation|SetWorldRotation (Variables|Default|GetCollision) "0, 0, 0" false false))

(fn ConstructionScript)