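; BP_RifaCharacter_Sample is a sample character Blueprint that adds a toggleable glide.
; Alternate presses of the glide input either zero vertical velocity, lowering gravity and raising air control, or restore normal values.
; A DoOnce reset after a short Delay throttles glide activation, which has no working falling check.
; Tick restores normal gravity and air control whenever the character moves on the ground, without resetting the FlipFlop.
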(event EventTick
  (params (DeltaSeconds :type Float%20%28single-precision%29))
  (bind _rifacharactermovement (Variables|Default|GetRifaCharacterMovement))
  (if (AI|Components|NavMovement|IsMovingonGround (Variables|Default|GetRifaCharacterMovement))
    (Variables|/Script/Engine.CharacterMovementComponent|SetGravityScale _rifacharactermovement 4.0)
    (Variables|/Script/Engine.CharacterMovementComponent|SetAirControl _rifacharactermovement 0.6)))

(event Input|ActionEvents|InputActionglide
  (params (Key :type Key%20Structure))
  (bind _rifacharactermovement (Variables|Default|GetRifaCharacterMovement))
  (bind _rifacharactermovement_2 (Variables|Default|GetRifaCharacterMovement))
  (bind _rifacharactermovement_3 (Variables|Default|GetRifaCharacterMovement))
  (:Pressed
    (Utilities|FlowControl|FlipFlop
      (:A
        (Utilities|FlowControl|DoOnce false :!label _label
          (:Completed
            (if true
              (Variables|/Script/Engine.MovementComponent|SetVelocity _rifacharactermovement_2 (Math|Vector|MakeVector (.x (Variables|/Script/Engine.MovementComponent|GetVelocity _rifacharactermovement_2)) (.y (Variables|/Script/Engine.MovementComponent|GetVelocity _rifacharactermovement_2)) 0.0))
              (Variables|/Script/Engine.CharacterMovementComponent|SetGravityScale _rifacharactermovement_3 0.07)
              (Variables|/Script/Engine.CharacterMovementComponent|SetAirControl _rifacharactermovement_3 0.7)
              (Utilities|FlowControl|Delay 0.2)
              (goto _label Reset)))))
      (:B
        (Variables|/Script/Engine.CharacterMovementComponent|SetGravityScale _rifacharactermovement 4.0)
        (Variables|/Script/Engine.CharacterMovementComponent|SetAirControl _rifacharactermovement 0.6)))))

(fn ConstructionScript)