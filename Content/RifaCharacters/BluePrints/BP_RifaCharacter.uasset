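; BP_RifaCharacter is a character Blueprint that lets the player interact with nearby objects through BP_InteractionInterface.
; InteractionSphere overlaps add and remove entries in InteractableInRange, using the actor if it implements the interface, otherwise its implementing components.
; The IA_Interact Enhanced Input action calls OnInteraction on the first entry in that array, passing the character, with no distance or priority sorting.
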(event OnComponentBeginOverlap(InteractionSphere)
  (params (OverlappedComponent :type Primitive%20Component%20Object%20Reference) (OtherActor :type Actor%20Object%20Reference) (OtherComp :type Primitive%20Component%20Object%20Reference) (OtherBodyIndex :type Integer) (bFromSweep :type Boolean) (SweepResult :type Hit%20Result%20Structure%20%28by%20ref%29))
  (bind _interactableinrange (Variables|Default|GetInteractableInRange))
  (bind _asbp_interaction_interface (Utilities|Casting|CastToBP_InteractionInterface OtherActor)
    (:then
      (Utilities|Array|AddUnique _interactableinrange _asbp_interaction_interface))
    (:CastFailed
      (for _array_element (Class|Actor|GetComponentsbyInterface OtherActor "/Game/BluePrint/UI/DialogSystem/BP_InteractionInterface.BP_InteractionInterface_C")
        (Utilities|Array|AddUnique _interactableinrange (.AsBP%20Interaction%20Interface (Utilities|Casting|CastToBP_InteractionInterface _array_element)))))))

(event OnComponentEndOverlap(InteractionSphere)
  (params (OverlappedComponent :type Primitive%20Component%20Object%20Reference) (OtherActor :type Actor%20Object%20Reference) (OtherComp :type Primitive%20Component%20Object%20Reference) (OtherBodyIndex :type Integer))
  (bind _interactableinrange (Variables|Default|GetInteractableInRange))
  (bind _asbp_interaction_interface (Utilities|Casting|CastToBP_InteractionInterface OtherActor)
    (:then
      (Utilities|Array|RemoveItem _interactableinrange _asbp_interaction_interface))
    (:CastFailed
      (for _array_element (Class|Actor|GetComponentsbyInterface OtherActor "/Game/BluePrint/UI/DialogSystem/BP_InteractionInterface.BP_InteractionInterface_C")
        (Utilities|Array|RemoveItem _interactableinrange (.AsBP%20Interaction%20Interface (Utilities|Casting|CastToBP_InteractionInterface _array_element)))))))

(event Input|EnhancedActionEvents|EnhancedInputActionIA_Interact
  (params (ActionValue :type Boolean) (ElapsedSeconds :type Float%20%28double-precision%29) (TriggeredSeconds :type Float%20%28double-precision%29) (InputAction :type Input%20Action%20Object%20Reference :default "/Game/RifaCharacters/Input/Actions/IA_Interact.IA_Interact"))
  (:Triggered
    (if (> (Utilities|Array|Length (Variables|Default|GetInteractableInRange)) 0)
      (Default|OnInteraction (Utilities|Array|Get(acopy) (Variables|Default|GetInteractableInRange)) self))))

(event EventBeginPlay)

(event Collision|EventActorBeginOverlap
  (params (OtherActor :type Actor%20Object%20Reference)))

(event EventTick
  (params (DeltaSeconds :type Float%20%28single-precision%29)))

(fn ConstructionScript)