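; Interactive object Blueprint that lets the player interact with it by pressing F while inside its trigger box.
; Overlapping the box enables input from player controller 0 and shows a prompt widget; leaving disables input and hides it.
; Pressing F calls DoInteraction, which hides the widget, turns off the box's collision and plays a 2D pickup sound.
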(event OnComponentBeginOverlap(Box)
  (params (OverlappedComponent :type Primitive%20Component%20Object%20Reference) (OtherActor :type Actor%20Object%20Reference) (OtherComp :type Primitive%20Component%20Object%20Reference) (OtherBodyIndex :type Integer) (bFromSweep :type Boolean) (SweepResult :type Hit%20Result%20Structure%20%28by%20ref%29))
  (Input|EnableInput (Game|GetPlayerController 0))
  (Rendering|SetVisibility (Variables|Default|GetWidget) true false))

(event OnComponentEndOverlap(Box)
  (params (OverlappedComponent :type Primitive%20Component%20Object%20Reference) (OtherActor :type Actor%20Object%20Reference) (OtherComp :type Primitive%20Component%20Object%20Reference) (OtherBodyIndex :type Integer))
  (Input|DisableInput (Game|GetPlayerController 0))
  (Rendering|SetVisibility (Variables|Default|GetWidget) false false))

(event Custom|DoInteraction
  (Rendering|SetVisibility (Variables|Default|GetWidget) false false)
  (Collision|SetCollisionEnabled (Variables|Default|GetBox) "NoCollision")
  (Audio|PlaySound2D "/Game/Sounds/Pickup_01.Pickup_01" 1.0 1.0 0.0 0 0))

(event Input|KeyboardEvents|F
  (params (Key :type Key%20Structure))
  (:Pressed
    (CallFunction|DoInteraction)))

(fn ConstructionScript)