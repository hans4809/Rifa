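; BP_Subtitle_01 is a one-time interactable prop with a configurable mesh and material that plays a subtitled sound.
; Overlapping its box enables input and shows a prompt widget; leaving reverses both.
; Pressing F, gated by DoOnce and a player-character check, hides the text and prompt, plays Subtitle_01 audio, shows WB_Subtitle using row "1" of SubtitleTable, and disables box collision.
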(event OnComponentBeginOverlap(Box)
  (params (OverlappedComponent :type Primitive%20Component%20Object%20Reference) (OtherActor :type Actor%20Object%20Reference) (OtherComp :type Primitive%20Component%20Object%20Reference) (OtherBodyIndex :type Integer) (bFromSweep :type Boolean) (SweepResult :type Hit%20Result%20Structure%20%28by%20ref%29))
  (Input|EnableInput (Game|GetPlayerController 0))
  (Rendering|SetVisibility (Variables|Default|GetWidget) true false))

(event OnComponentEndOverlap(Box)
  (params (OverlappedComponent :type Primitive%20Component%20Object%20Reference) (OtherActor :type Actor%20Object%20Reference) (OtherComp :type Primitive%20Component%20Object%20Reference) (OtherBodyIndex :type Integer))
  (Input|DisableInput (Game|GetPlayerController 0))
  (Rendering|SetVisibility (Variables|Default|GetWidget) false false))

(event EventBeginPlay
  (Components|StaticMesh|SetStaticMesh (Variables|Default|GetStaticMesh) (Variables|Default|GetMesh)))

(event Input|KeyboardEvents|F
  (params (Key :type Key%20Structure))
  (:Pressed
    (Utilities|FlowControl|DoOnce false
      (:Completed
        (if (== (stale OnComponentBeginOverlap(Box) OtherActor) (Game|GetPlayerCharacter 0))
          (Rendering|SetVisibility (Variables|Default|GetTextRender) false false)
          (Audio|PlaySound2D "/Game/Blueprints/Subtitle_01.Subtitle_01" 1.0 1.0 0.0 0 0)
          (bind _returnvalue (UserInterface|CreateWidget "/Game/Subtitle/Master/WB_Subtitle.WB_Subtitle_C" 0 (Utilities|Struct|MakeDataTableRowHandle (Variables|Default|GetSubtitleTable) "1")))
          (UserInterface|Viewport|AddtoViewport _returnvalue 0)
          (Collision|SetCollisionEnabled (Variables|Default|GetBox) "NoCollision"))))))

(fn ConstructionScript
  (Rendering|Material|SetMaterial (Variables|Default|GetStaticMesh) 0 (Variables|Default|GetMaterial))
  (Components|StaticMesh|SetStaticMesh (Variables|Default|GetStaticMesh) (Variables|Default|GetMesh)))