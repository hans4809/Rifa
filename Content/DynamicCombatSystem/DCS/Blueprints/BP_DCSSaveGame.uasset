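; Save game object for the Dynamic Combat System that stores and restores an actor's inventory, equipment, selected main hand type and stats.
; SaveData reads the actor's inventory, equipment and stats manager components, resetting each slot's hidden flag and keeping only tag and base value per stat.
; LoadData writes the saved data back through those components' setters, applying stats one by one by tag.
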(fn SaveData
  (params (Actor :type Actor%20Object%20Reference))
  (bind _returnvalue (Actor|GetComponentbyClass Actor "/Game/DynamicCombatSystem/DCS/Blueprints/Components/Inventory/BP_EquipmentComponent.BP_EquipmentComponent_C"))
  (Utilities|FlowControl|Sequence
    (:then_0
      ;[1 0 0] save inventory
      (Variables|Default|SetInventory (Variables|/Game/DynamicCombatSystem/DCS/Blueprints/Components/Inventory/BP_InventoryComponent.BP_InventoryComponent_C|GetInventory (Actor|GetComponentbyClass Actor "/Game/DynamicCombatSystem/DCS/Blueprints/Components/Inventory/BP_InventoryComponent.BP_InventoryComponent_C"))))
    (:then_1
      ;[1 0 0] save equipment
      (Utilities|FlowControl|Sequence
        (:then_0
          (bind _equipment (Default|GetSlotsasArray _returnvalue))
          (bind _output_get (Variables|Default|SetEquipment _equipment))
          ;;[0 0 0] don't save hidden or displayed item value, it will be auto generated upon loading
          (for (_ _array_index) _output_get
            (for (_ _array_index_2) (.Slots (Utilities|Struct|BreakF_EquipmentSlots (Utilities|Array|Get(acopy) _output_get _array_index)))
              (Utilities|Struct|SetmembersinF_EquipmentSlot (Utilities|Array|Get(acopy) (.Slots (Utilities|Struct|BreakF_EquipmentSlots (Utilities|Array|Get(acopy) _output_get _array_index))) _array_index_2) false 0))))
        (:then_1
          (Variables|Default|SetSelectedHandType (Default|GetSelectedMainHandType _returnvalue)))))
    (:then_2
      ;[1 0 0] save stats
      (Utilities|Array|Clear (Variables|Default|GetStats))
      (for _array_element (Variables|/Game/DynamicCombatSystem/DCS/Blueprints/Components/StatsManager/BP_StatsManagerComponent.BP_StatsManagerComponent_C|GetStats (Actor|GetComponentbyClass Actor "/Game/DynamicCombatSystem/DCS/Blueprints/Components/StatsManager/BP_StatsManagerComponent.BP_StatsManagerComponent_C"))
        (Utilities|Array|Add (Variables|Default|GetStats) (Utilities|Struct|MakeF_Stat (.AttributeTag (Utilities|Struct|BreakF_Stat _array_element)) (.BaseValue (Utilities|Struct|BreakF_Stat _array_element)))) ; save only tag + base value
      ))))

(fn LoadData
  (params (Actor :type Actor%20Object%20Reference))
  (bind _returnvalue (Actor|GetComponentbyClass Actor "/Game/DynamicCombatSystem/DCS/Blueprints/Components/Inventory/BP_EquipmentComponent.BP_EquipmentComponent_C"))
  (Utilities|FlowControl|Sequence
    (:then_0
      ;[1 0 0] load inventory
      (Default|SetInventory (Actor|GetComponentbyClass Actor "/Game/DynamicCombatSystem/DCS/Blueprints/Components/Inventory/BP_InventoryComponent.BP_InventoryComponent_C") (Variables|Default|GetInventory)))
    (:then_1
      ;[1 0 0] load equipment
      (Default|SetEquipment _returnvalue (Variables|Default|GetEquipment))
      (Default|SetMainHandType _returnvalue (Variables|Default|GetSelectedHandType)))
    (:then_2
      ;[1 0 0] load stats
      (for _array_element (Variables|Default|GetStats)
        (Default|SetStat (Actor|GetComponentbyClass Actor "/Game/DynamicCombatSystem/DCS/Blueprints/Components/StatsManager/BP_StatsManagerComponent.BP_StatsManagerComponent_C") (.AttributeTag (Utilities|Struct|BreakF_Stat _array_element)) (.BaseValue (Utilities|Struct|BreakF_Stat _array_element)))))))