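; Montage manager actor component in the Dynamic Combat System that maps action gameplay tags to animation montages.
; Lookups ask the owner through I_MontageManagerComponent for a data table, scan its rows for an exact tag match, then fall back to a default table.
; Helpers return a montage by index, the last index or a random index, and each lookup records the last requested action for later queries.
; BeginPlay prints a warning if the owner lacks the interface.
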(event EventBeginPlay
  (if (not (Utilities|DoesObjectImplementInterface (Components|GetOwner) "/Game/DynamicCombatSystem/DCS/Blueprints/Interfaces/I_MontageManagerComponent.I_MontageManagerComponent_C"))
    (Development|PrintString (Utilities|String|Append "Warning! " (Utilities|GetClassDisplayName (Utilities|GetClass (Components|GetOwner))) " does not implement interface I_MontageManager") true true "(R=1.000000,G=0.974717,B=0.000000,A=1.000000)" 5.0)))

(fn GetMontageforAction
  (params (ActionTag :type Gameplay%20Tag%20Structure) (Index :type Integer))
  (bind (_isfound _action) (CallFunction|GetAction ActionTag))
  (if _isfound
    (if (Utilities|Array|IsValidIndex (.Montages (Utilities|Struct|BreakF_MontageAction _action)) Index)
      (return (Utilities|Array|Get(acopy) (.Montages (Utilities|Struct|BreakF_MontageAction _action)) Index))
      (else
        (return 0)))
    (else
      (return 0))))

(fn GetMontageActionLastIndex
  (params (ActionTag :type Gameplay%20Tag%20Structure))
  (bind (_isfound _action) (CallFunction|GetAction ActionTag))
  (if _isfound
    (return (Utilities|Array|LastIndex (Utilities|Struct|BreakF_MontageAction _action)))
    (else
      (return -1))))

(fn GetRandomMontageIndex
  (params (ActionTag :type Gameplay%20Tag%20Structure))
  (return (Math|Random|RandomIntegerinRange 0 (CallFunction|GetMontageActionLastIndex ActionTag))))

(fn GetLastRequestedAction
  (return (Variables|Default|GetLastRequestedAction)))

(fn GetAction
  (params (ActionTag :type Gameplay%20Tag%20Structure))
  (bind _output_get (Variables|Default|SetLastRequestedAction ActionTag))
  (bind _montages (Class|IMontageManagerComponent|GetMontages(Message) (Components|GetOwner) _output_get))
  (bind (_isfound _out_row) (CallFunction|GetActionfromTable _montages ActionTag))
  (if _isfound
    (return _isfound _out_row)
    (else
      (bind (_isfound_2 _out_row_2) (CallFunction|GetActionfromTable (Variables|Default|GetDefaultMontageActionsDataTable) ActionTag))
      (return _isfound_2 _out_row_2))))

(fn GetActionfromTable
  (params (TableToSearch :type Data%20Table%20Object%20Reference) (ActionTag :type Gameplay%20Tag%20Structure))
  (Utilities|IsValid TableToSearch
    (:Is%20Valid
      (bind _outrownames (DataTable|GetDataTableRowNames TableToSearch))
      (for _array_element _outrownames
        (bind _returnvalue (Utilities|GetDataTableRow TableToSearch _array_element)
          (:then
            (if (GameplayTags|MatchesTag (Utilities|Struct|BreakF_MontageAction _returnvalue) ActionTag true)
              (return true _returnvalue)))
          (:RowNotFound
            (return false "")))))
    (:Is%20Not%20Valid
      _))
  (return false ""))

(fn WasLastRequestedAction
  (params (ActionTag :type Gameplay%20Tag%20Structure) (bExactMatch :type Boolean))
  (return (GameplayTags|MatchesTag (CallFunction|GetLastRequestedAction) ActionTag bExactMatch)))