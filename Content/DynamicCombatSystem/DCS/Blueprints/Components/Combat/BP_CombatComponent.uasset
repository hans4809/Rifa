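; Actor component that holds its owner's combat state: combat style tag, weapon type, melee attack and combo, bow, block and gun data.
; Style, weapon and gun setters notify on change, while magazine ammo is cached per gun ID.
; Shots add curve-driven heat that cools on tick and sets spread, adjusted by movement, zoom and crouch.
; A helper sphere-traces along a spread-adjusted view ray to aim projectiles from their spawn point.
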(event EventBeginPlay
  (CallFunction|UpdateReferences)
  (if (Variables|Settings|GetbDebug)
    (Components|Tick|SetComponentTickEnabled true)))

(event EventTick
  (params (DeltaSeconds :type Float%20%28single-precision%29))
  (Guns|TickGunData DeltaSeconds)
  (if (Variables|Settings|GetbDebug)
    (CallFunction|DebugTick DeltaSeconds)))

(fn HasShield
  (|SwitchGameplayTag (Variables|Settings|GetCombatStyleTag)
    (:Default
      (return false))
    (:CombatStyle.Melee.Armed.OneHandedWeapon.Shield
      _)
    (:CombatStyle.Melee.Unarmed.Shield
      _)
    (:CombatStyle.Ranged.Magic.Shield
      _))
  (return true))

(fn HasArrows
  (return (Variables|Settings|GetbHasArrows)))

(fn GetCombatStyle
  (return (Variables|Settings|GetCombatStyleTag)))

(fn IsCombatStyle
  (params (CombatStyleTag :type Gameplay%20Tag%20Container%20Structure))
  (return (GameplayTags|MatchesAnyTags (Variables|Settings|GetCombatStyleTag) CombatStyleTag)))

(fn SetCombatStyle
  (params (NewCombatStyleTag :type Gameplay%20Tag%20Structure))
  (if (!= NewCombatStyleTag (Variables|Settings|GetCombatStyleTag))
    ;[1 0 0] Update current combat style and call event
    (LocalVariables|SetL_PreviousCombatStyle (Variables|Settings|GetCombatStyleTag))
    (bind _output_get (Variables|Settings|SetCombatStyleTag NewCombatStyleTag))
    (Default|CallOnCombatStyleChanged (LocalVariables|GetL_PreviousCombatStyle) _output_get)))

(fn SetComboCounter
  (params (NewComboCounter :type Integer) (AutoResetDelay :type Float%20%28double-precision%29))
  (Variables|Melee|SetComboCounter NewComboCounter)
  (if (> AutoResetDelay 0.0)
    ;[1 0 0] auto reset combo counter if time was given
    (ComboCounter|ResetComboCounterwithDelay AutoResetDelay)
    (else
      ;[1 0 0] stop timer reseting combo counter
      ; if it was running
      (Utilities|Time|ClearandInvalidateTimerbyHandle (Variables|Melee|GetTimerHandle_ResetComboCounter)))))

(fn ResetComboCounter
  (Variables|Melee|SetComboCounter 0))

(fn GetComboCounter
  (return (Variables|Melee|GetComboCounter)))

(fn ResetComboCounterwithDelay
  (params (Delay :type Float%20%28double-precision%29))
  (if (> Delay 0.0)
    (bind _returnvalue (Utilities|Time|SetTimerbyEvent (EventDispatchers|CreateEvent :!event ResetComboCounter) Delay))
    (Variables|Melee|SetTimerHandle_ResetComboCounter _returnvalue)
    (else
      (ComboCounter|ResetComboCounter))))

(fn IsZooming
  (return (> (Variables|Archery|GetZoomAlpha) 0.0)))

(fn GetBowProjectileClass
  (return (Variables|Settings|GetBowProjectileClass)))

(fn SetWeaponType
  (params (NewWeaponType :type E_WeaponType%20Enum :default "NewEnumerator5"))
  (bind _weapontype (WeaponType|GetWeaponType))
  (if (Utilities|Enum|NotEqual(Enum) NewWeaponType _weapontype)
    (bind _output_get (LocalVariables|SetL_PreviousWeaponType _weapontype))
    (bind _output_get_2 (Variables|Settings|SetWeaponType NewWeaponType))
    (Default|CallOnWeaponTypeChanged _output_get _output_get_2)))

(fn GetWeaponType
  (return (Variables|Settings|GetWeaponType)))

(fn SetBowProjectileClass
  (params (NewProjectileClass :type BP%20Base%20Projectile%20Class%20Reference))
  (Variables|Settings|SetBowProjectileClass NewProjectileClass))

(fn SetHasArrows
  (params (NewHasArrows :type Boolean))
  (Variables|Settings|SetbHasArrows NewHasArrows))

(fn SetDrawBowAlpha
  (params (NewAlpha :type Float%20%28double-precision%29))
  (Variables|Archery|SetDrawBowAlpha NewAlpha))

(fn SetBlockAlpha
  (params (NewAlpha :type Float%20%28double-precision%29))
  (Variables|Melee|SetBlockAlpha NewAlpha))

(fn GetDrawBowAlpha
  (return (Variables|Archery|GetDrawBowAlpha)))

(fn GetBlockAlpha
  (return (Variables|Melee|GetBlockAlpha)))

(fn SetMeleeAttackType
  (params (NewMeleeAttackType :type E_MeleeAttackType%20Enum :default "NewEnumerator6"))
  (Variables|Melee|SetMeleeAttackType NewMeleeAttackType))

(fn GetMeleeAttackType
  (return (Variables|Melee|GetMeleeAttackType)))

(fn IsMeleeAttackType
  (params (AttackTypeToCheck :type E_MeleeAttackType%20Enum :default "NewEnumerator6"))
  (return (Utilities|Enum|Equal(Enum) AttackTypeToCheck (Attack|GetMeleeAttackType))))

(fn UpdateReferences
  (bind _as캐릭터 (Utilities|Casting|CastToCharacter (Components|GetOwner)))
  (Variables|Default|SetOwnerAsCharacter _as캐릭터))

(fn DebugTick
  (params (DeltaTime :type Float%20%28double-precision%29))
  (Utilities|FlowControl|Sequence
    (:then_0
      (if (!= (Utilities|Struct|BreakF_GunWeaponData (Variables|Guns|GetCurrentGunData)) "") ; is current gun valid?
        ;[1 0 0] show heat & spread of current gun
        (Development|PrintText (Utilities|Text|FormatText "Gun Heat: {heat} Spread Angle: {spread}" (Variables|Guns|GetCurrentGunHeat) (Guns|Spread|GetCurrentGunSpreadAngle)) true false "(R=0.558249,G=0.255208,B=1.000000,A=1.000000)" DeltaTime "")))
    (:then_1
      ;[1 0 0] show current combat style & weapon type
      (Development|PrintText (Utilities|Text|FormatText "{owner}: CombatStyle: {CombatStyleTag} | Weapon: {weapon}" (Components|GetOwner) (GameplayTags|GetDebugStringfromGameplayTag (Variables|Settings|GetCombatStyleTag)) (Utilities|String|EnumtoString (Variables|Settings|GetWeaponType))) true false "(R=0.428879,G=0.037092,B=1.000000,A=1.000000)" DeltaTime ""))))

(fn HasAmmoinInventory
  (return (Variables|Settings|GetbHasAmmoInInventory)))

(fn SetHasAmmoinInventory
  (params (NewHasAmmo :type Boolean))
  (Variables|Settings|SetbHasAmmoInInventory NewHasAmmo))

(fn UpdateCachedMagazineAmmoData
  (params (AmmoData :type F%20Cached%20Ammo%20Data%20Structure))
  (bind (_gunid _currentammo) (Utilities|Struct|BreakF_CachedAmmoData AmmoData))
  (bind _cachedammodata (Variables|Guns|GetCachedAmmoData))
  ;[1 0.573 0] is ammo for this gun already cached?
  (bind (_found _index) (Guns|Ammo|FindMagazineAmmoData _gunid))
  (if _found
    ;[1 0.573 0] update ammo value
    (Utilities|Struct|SetmembersinF_CachedAmmoData (Utilities|Array|Get(acopy) _cachedammodata _index) _currentammo)
    (else
      ;[1 0.573 0] add ammo as new cuz it wasn't saved before
      (Utilities|Array|Add _cachedammodata AmmoData))))

(fn FindMagazineAmmoData
  (params (GunId :type Name))
  ;[1 0.573 0] Search for cached ammo by gun Id
  (for (_array_element _array_index) (Variables|Guns|GetCachedAmmoData)
    (if (== (Utilities|Struct|BreakF_CachedAmmoData _array_element) GunId)
      (return true _array_index _array_element)))
  (return false -1 ""))

(fn SetCurrentGunData
  (params (NewGunId :type F%20Gun%20Weapon%20Data%20Structure%20%28by%20ref%29))
  (if (!= (Utilities|Struct|BreakF_GunWeaponData NewGunId) (Utilities|Struct|BreakF_GunWeaponData (Variables|Guns|GetCurrentGunData))) ; is new gun different than current one?
    (bind _output_get (Variables|Guns|SetCurrentGunData NewGunId))
    (Guns|Spread|SetCurrenGunHeat (Math|Float|SafeDivide (.MaxHeat (Guns|Spread|GetCurrentGunHeatRange)) 2.0)) ; set half of max heat on switching weapon
    (Utilities|FlowControl|Sequence
      (:then_0
        ;[1 0.573 0] If this gun is new, and doesn't have ammo data saved yet
        ; it means that it is used for the first time, set full magazine ammo
        (bind _found (Guns|Ammo|FindMagazineAmmoData (.GunUniqueName (Utilities|Struct|BreakF_GunWeaponData _output_get))))
        (if (not _found)
          (Guns|Ammo|UpdateCachedMagazineAmmoData (Utilities|Struct|MakeF_CachedAmmoData (.GunUniqueName (Utilities|Struct|BreakF_GunWeaponData _output_get)) (.MaxMagazineAmmo (Utilities|Struct|BreakF_GunWeaponData _output_get))))))
      (:then_1
        (Default|CallOnGunDataChanged (Variables|Guns|GetCurrentGunData) (Guns|Ammo|GetAmmoinCurrentGun) true)))))

(fn SetCurrentGunMagazineAmmo
  (params (NewAmmo :type Integer))
  ;[1 0.573 0] just update ammo value for current gun id
  (Guns|Ammo|UpdateCachedMagazineAmmoData (Utilities|Struct|MakeF_CachedAmmoData (Utilities|Struct|BreakF_GunWeaponData (Variables|Guns|GetCurrentGunData)) NewAmmo))
  (Default|CallOnGunDataChanged (Variables|Guns|GetCurrentGunData) (Guns|Ammo|GetAmmoinCurrentGun) false))

(fn GetAmmoinCurrentGun
  ;[1 0.573 0] search for ammo by current gun id
  (bind (_found _index _ammodata) (Guns|Ammo|FindMagazineAmmoData (Utilities|Struct|BreakF_GunWeaponData (Variables|Guns|GetCurrentGunData))))
  ;[1 0.573 0] return ammo value if found or 0 if not
  (if _found
    (return (Utilities|Struct|BreakF_CachedAmmoData _ammodata))
    (else
      (return 0))))

(fn GetMaxAmmoinCurrentGun
  (return (Utilities|Struct|BreakF_GunWeaponData (Variables|Guns|GetCurrentGunData))))

(fn HasAmmoinCurrentGunMagazine
  (return (> (Guns|Ammo|GetAmmoinCurrentGun) 0)))

(fn AddGunShotHeat
  ;[1 0.573 0] how much heat should be added
  (bind _output_get (LocalVariables|SetL_HeatPerShot (Guns|Spread|ConvertHeattoHeatPerShot (Variables|Guns|GetCurrentGunHeat))))
  (Guns|Spread|SetCurrenGunHeat (+ _output_get (Variables|Guns|GetCurrentGunHeat)))
  ;[1 0.573 0] update time the gun was fired
  (Variables|Guns|SetLastGunFireTime (Utilities|Time|GetTimeSeconds)))

(fn UpdateGunHeat
  (params (DeltaTime :type Float%20%28double-precision%29))
  (bind _currentgundata (Variables|Guns|GetCurrentGunData))
  (bind (_heattocooldownpersecond _heatrecoverycooldowndelay) (Utilities|Struct|BreakF_GunWeaponData _currentgundata))
  (if (> (Variables|Guns|GetCurrentGunHeat) 0.0) ; has any gun heat to reduce?
    ;[1 0.573 0] should start cooling down gun heat?
    (bind _output_get (LocalVariables|SetL_TimeSinceFired (- (Utilities|Time|GetTimeSeconds) (Variables|Guns|GetLastGunFireTime))))
    (if (> _output_get _heatrecoverycooldowndelay)
      (bind _output_get_2 (LocalVariables|SetL_CooldownRate _heattocooldownpersecond)) ; how much heat to remove per second
      (Guns|Spread|SetCurrenGunHeat (- (Variables|Guns|GetCurrentGunHeat) (* _output_get_2 DeltaTime))))))

(fn GetCurrentGunSpreadAngle
  (Utilities|FlowControl|Sequence
    (:then_0
      ;[1 0.573 0] Is first shot? means is gun heat at lowest possible value?
      (LocalVariables|SetL_IsFirstShot (and (Utilities|Struct|BreakF_GunWeaponData (Variables|Guns|GetCurrentGunData)) (Math|Float|NearlyEqual(Float) (.MinHeat (Guns|Spread|GetCurrentGunHeatRange)) (Variables|Guns|GetCurrentGunHeat) 1e-06))))
    (:then_1
      (bind _output_get (LocalVariables|SetL_FinalSpread (Math|Float|SelectFloat 0.0 (Variables|Guns|GetCurrentGunSpreadAngle) (LocalVariables|GetL_IsFirstShot))))
      (bind _output_get_2 (LocalVariables|SetL_FinalSpread (+ _output_get (Variables|Guns|GetCurrentMoveSpeedSpreadAngle))))
      (return (* _output_get_2 (Variables|Guns|GetCurrentZoomSpreadMultiplier) (Variables|Guns|GetCurrentCrouchSpreadMultiplier))))))

(fn SetCurrenGunHeat
  (params (NewHeat :type Float%20%28double-precision%29))
  (bind (_minheat _maxheat) (Guns|Spread|GetCurrentGunHeatRange))
  ;[1 0.573 0] calculate new heat and check if it has changed
  (bind _output_get (LocalVariables|SetL_ClampedHeat (Math|Float|Clamp(Float) NewHeat _minheat _maxheat)))
  (if (!= _output_get (Variables|Guns|GetCurrentGunHeat))
    (LocalVariables|SetL_Delta (- (Variables|Guns|GetCurrentGunHeat) (LocalVariables|GetL_ClampedHeat)))
    (bind _output_get_2 (Variables|Guns|SetCurrentGunHeat (LocalVariables|GetL_ClampedHeat)))
    (Variables|Guns|SetCurrentGunSpreadAngle (Guns|Spread|ConvertGunHeattoSpreadAngle _output_get_2))
    (Default|CallOnGunHeatChanged (Variables|Guns|GetCurrentGunHeat) (LocalVariables|GetL_Delta))))

(fn GetDirectiontoSpawnProjectile
  (params (SpawnLocation :type Vector) (ViewLocation :type Vector) (ViewDirection :type Vector) (MaxRange :type Float%20%28double-precision%29) (SpreadAngleDeg :type Float%20%28double-precision%29) (SpreadExponent :type Float%20%28double-precision%29) (TraceRadius :type Float%20%28double-precision%29))
  (Utilities|FlowControl|Sequence
    (:then_0
      ;[1 0.573 0] calculate trace start point
      (LocalVariables|SetL_LineTraceStart (+ ViewLocation (* ViewDirection (Math|Vector|VectorLength (- SpawnLocation ViewLocation))))))
    (:then_1
      ;[1 0.573 0] calculate trace end point
      (LocalVariables|SetL_LineTraceEnd (+ (LocalVariables|GetL_LineTraceStart) (* (CallFunction|AddSpreadtoDirVector ViewDirection SpreadExponent SpreadAngleDeg) MaxRange))))
    (:then_2
      ;[1 0.573 0] Get initial spawn direction
      (LocalVariables|SetL_OutDirection (Math|Vector|GetUnitDirection(Vector) SpawnLocation (LocalVariables|GetL_LineTraceEnd))))
    (:then_3
      (bind _outhits (Collision|MultiSphereTraceByChannel (LocalVariables|GetL_LineTraceStart) (LocalVariables|GetL_LineTraceEnd) TraceRadius (CallFunction|GetProjectileChannel) false (Utilities|Array|MakeArray (Components|GetOwner)) "None" true "(R=1.000000,G=0.000000,B=0.000000,A=1.000000)" "(R=0.000000,G=1.000000,B=0.000000,A=1.000000)" 2.0))
      (for _array_element _outhits
        ;[1 0.573 0] each actor can be checked only once
        (bind _returnvalue (Utilities|Array|AddUnique (LocalVariables|GetL_HitActors) (.HitActor (Collision|BreakHitResult _array_element))))
        (if (>= _returnvalue 0)
          (LocalVariables|SetL_OutDirection (Math|Vector|GetUnitDirection(Vector) SpawnLocation (.ImpactPoint (Collision|BreakHitResult _array_element))))
          (return SpawnLocation (LocalVariables|GetL_OutDirection))))
      (return SpawnLocation (LocalVariables|GetL_OutDirection)))))

(fn UpdateSpreadMultipliers
  (params (DeltaTime :type Float%20%28double-precision%29))
  (Utilities|FlowControl|Sequence
    (:then_0
      ;[1 0.573 0] Update move speed spread angle
      (bind _ownerascharacter (Variables|Default|GetOwnerAsCharacter)
        (:then
          (Variables|Guns|SetCurrentMoveSpeedSpreadAngle (Math|Interpolation|FInterpTo (Variables|Guns|GetCurrentMoveSpeedSpreadAngle) (Guns|Spread|ConvertMoveSpeedtoSpreadAngle (Math|Vector|VectorLength (Transformation|GetVelocity _ownerascharacter))) DeltaTime 5.0)))
        (:else)))
    (:then_1
      ;[1 0.573 0] Update zoom spread angle multiplier
      (Variables|Guns|SetCurrentZoomSpreadMultiplier (Math|Float|MapRangeClamped (Variables|Archery|GetZoomAlpha) 0.0 1.0 1.0 (Utilities|Struct|BreakF_GunWeaponData (Variables|Guns|GetCurrentGunData)))))
    (:then_2
      ;[1 0.573 0] Update crouch spread multiplier
      (bind _ownerascharacter_2 (Variables|Default|GetOwnerAsCharacter)
        (:then
          (Variables|Guns|SetCurrentCrouchSpreadMultiplier (Math|Interpolation|FInterpTo (Variables|Guns|GetCurrentCrouchSpreadMultiplier) (select (AI|Components|NavMovement|IsCrouching (Variables|/Script/Engine.Character|GetCharacterMovement _ownerascharacter_2)) (Utilities|Struct|BreakF_GunWeaponData (Variables|Guns|GetCurrentGunData)) 1.0) DeltaTime 5.0)))
        (:else)))))

(fn GetCurrentGunHeatRange
  (bind _currentgundata (Variables|Guns|GetCurrentGunData))
  (bind _heattospreadcurve (Utilities|Struct|BreakF_GunWeaponData _currentgundata))
  (bind (_mintime _maxtime) (Math|Curves|GetTimeRange _heattospreadcurve))
  (if (!= _heattospreadcurve 0)
    (return _mintime _maxtime)
    (else
      (return 0.0 0.0))))

(fn ConvertMoveSpeedtoSpreadAngle
  (params (MoveSpeed :type Float%20%28double-precision%29))
  (bind _currentgundata (Variables|Guns|GetCurrentGunData))
  (bind _movespeedtospreadcurve (Utilities|Struct|BreakF_GunWeaponData _currentgundata))
  (if (!= _movespeedtospreadcurve 0)
    (return (Math|Curves|GetFloatValue _movespeedtospreadcurve MoveSpeed))
    (else
      (return 0.0))))

(fn ConvertGunHeattoSpreadAngle
  (params (GunHeat :type Float%20%28double-precision%29))
  (bind _currentgundata (Variables|Guns|GetCurrentGunData))
  (bind _heattospreadcurve (Utilities|Struct|BreakF_GunWeaponData _currentgundata))
  (if (!= _heattospreadcurve 0)
    (return (Math|Curves|GetFloatValue _heattospreadcurve GunHeat))
    (else
      (return 0.0))))

(fn ConvertHeattoHeatPerShot
  (params (Heat :type Float%20%28single-precision%29))
  (bind _currentgundata (Variables|Guns|GetCurrentGunData))
  (bind _heattoheatpershotcurve (Utilities|Struct|BreakF_GunWeaponData _currentgundata))
  (Utilities|IsValid _heattoheatpershotcurve
    (:Is%20Valid
      (return (Math|Curves|GetFloatValue _heattoheatpershotcurve Heat)))
    (:Is%20Not%20Valid
      (return 0.0))))

(fn GetGunProjectileClass
  (return (Utilities|Struct|BreakF_GunWeaponData (Variables|Guns|GetCurrentGunData))))

(fn GetGunCrosshairClass
  (return (Utilities|Struct|BreakF_GunWeaponData (Variables|Guns|GetCurrentGunData))))

(fn TickGunData
  (params (DeltaTime :type Float%20%28double-precision%29))
  (if (!= (Utilities|Struct|BreakF_GunWeaponData (Variables|Guns|GetCurrentGunData)) "") ; update only if gun item is set
    (Guns|Spread|UpdateGunHeat DeltaTime)
    (Guns|Spread|UpdateSpreadMultipliers DeltaTime)))