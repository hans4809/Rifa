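; Stats regenerator for the DCS stats manager that restores one gameplay-tagged stat toward its tagged maximum, as configured by RegenData.
; Stat change events start a looping timer that adds the multiplied regen value each interval, capped at max, and stops once full.
; A drop in the maximum clamps the current value down.
; Regeneration can be paused indefinitely or for a duration, after which a timer resumes it.
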(fn GetStatsValues
  (bind _regendata (Variables|Settings|GetRegenData))
  (bind _statsmanagercomponent (Variables|Default|GetStatsManagerComponent))
  (bind (_currentvalueattributetag _maxvalueattributetag) (Utilities|Struct|BreakF_StatRegenData _regendata))
  (return (Default|GetStatValue _statsmanagercomponent _currentvalueattributetag true) (Default|GetStatValue _statsmanagercomponent _maxvalueattributetag true)))

(fn OnStatChanged
  (params (ChangedStat :type Gameplay%20Tag%20Structure) (StatValue :type Float%20%28double-precision%29) (Delta :type Float%20%28double-precision%29) (IsDeltaNegative :type Boolean))
  (Utilities|FlowControl|Sequence
    (:then_0
      ;[1 0 0] Observe MaxValue stat
      (if (GameplayTags|MatchesTag ChangedStat (Utilities|Struct|BreakF_StatRegenData (Variables|Settings|GetRegenData)) true) ; Has max value stat changed?
        (if IsDeltaNegative ; Has its value decreased?
          (bind (_currentvalue _maxvalue) (CallFunction|GetStatsValues))
          (if (> _currentvalue _maxvalue)
            (Default|SetStat (Variables|Default|GetStatsManagerComponent) (Utilities|Struct|BreakF_StatRegenData (Variables|Settings|GetRegenData)) _maxvalue))
          (else
            (LocalVariables|SetL_StartRegen true)))))
    (:then_1
      ;[1 0 0] Observer CurrentValue stat
      (if (GameplayTags|MatchesTag ChangedStat (Utilities|Struct|BreakF_StatRegenData (Variables|Settings|GetRegenData)) true) ; Has current stat value changed?
        (LocalVariables|SetL_StartRegen true)))
    (:then_2
      (if (LocalVariables|GetL_StartRegen)
        (CallFunction|StartRegenerationTimer)))))

(fn RegenerationLoop
  (bind (_currentvalue _maxvalue) (CallFunction|GetStatsValues))
  (LocalVariables|SetL_CurrentValue _currentvalue)
  (LocalVariables|SetL_MaxValue _maxvalue)
  (if (< (LocalVariables|GetL_CurrentValue) (LocalVariables|GetL_MaxValue))
    (LocalVariables|SetL_RegenValue (CallFunction|GetRegenValue))
    (Utilities|FlowControl|Sequence
      (:then_0
        ;[1 0 0] Calculate value to regen
        (if (> (+ (LocalVariables|GetL_RegenValue) (LocalVariables|GetL_CurrentValue)) (LocalVariables|GetL_MaxValue)) ; clamp regen value to not\nexceed stat MaxValue
          (LocalVariables|SetL_RegenValue (- (LocalVariables|GetL_MaxValue) (LocalVariables|GetL_CurrentValue)))))
      (:then_1
        ;[1 0 0] Modify value
        (Default|ModifyStat (Variables|Default|GetStatsManagerComponent) (Utilities|Struct|BreakF_StatRegenData (Variables|Settings|GetRegenData)) (LocalVariables|GetL_RegenValue))))
    (else
      ;[1 0 0] stop regen if already at max
      (CallFunction|StopRegenerationTimer))))

(fn StartRegenerationTimer
  ;[1 0 0] Check if can run regen timer
  (if (and (not (Utilities|Time|IsValidTimerHandle (Variables|Default|GetTimerHandle_RegenerationLoop))) (not (Variables|Default|GetIsRegenerationPaused)))
    (bind _returnvalue (Utilities|Time|SetTimerbyEvent (EventDispatchers|CreateEvent :!event RegenerationLoop) (Utilities|Struct|BreakF_StatRegenData (Variables|Settings|GetRegenData)) true))
    (Variables|Default|SetTimerHandle_RegenerationLoop _returnvalue)))

(fn StopRegenerationTimer
  (Utilities|Time|ClearandInvalidateTimerbyHandle (Variables|Default|GetTimerHandle_RegenerationLoop)))

(fn Init
  ;[1 0 0] Observe stat changed event on owning stats manager component
  (EventDispatchers|BindEventtoOnStatChanged (Variables|Default|GetStatsManagerComponent) (EventDispatchers|CreateEvent :!event OnStatChanged)))

(fn PauseRegeneration
  (params (Duration :type Float%20%28double-precision%29))
  (Utilities|FlowControl|Sequence
    (:then_0
      ;[1 0 0] Stop regen timer
      (Variables|Default|SetIsRegenerationPaused true)
      (CallFunction|StopRegenerationTimer)
      (Utilities|Time|ClearandInvalidateTimerbyHandle (Variables|Default|GetTimerHandle_ResumeRegeneration)))
    (:then_1
      ;[1 0 0] Resume regen timer after duration
      (if (> Duration 0.0)
        (bind _returnvalue (Utilities|Time|SetTimerbyEvent (EventDispatchers|CreateEvent :!event ResumeRegeneration) Duration))
        (Variables|Default|SetTimerHandle_ResumeRegeneration _returnvalue)))))

(fn ResumeRegeneration
  (Utilities|Time|ClearandInvalidateTimerbyHandle (Variables|Default|GetTimerHandle_ResumeRegeneration))
  (Variables|Default|SetIsRegenerationPaused false)
  (CallFunction|StartRegenerationTimer))

(fn GetRegenValue
  (bind _regendata (Variables|Settings|GetRegenData))
  (bind (_regenvalue _regenvaluemultiplier) (Utilities|Struct|BreakF_StatRegenData _regendata))
  (return (* _regenvalue _regenvaluemultiplier)))

(fn SetRegenData
  (params (RegenData :type F%20Stat%20Regen%20Data%20Structure%20%28by%20ref%29))
  (Variables|Settings|SetRegenData RegenData))