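; BP_DI_BaseSpell is the base displayed item for spells in the combat system, showing a spell as a hand particle effect.
; The construction script applies the HandParticle template to its particle component.
; The Attach override activates the particle and defers to parent attachment only when the item is visible and its owner is in combat.
; Otherwise it deactivates the particle and reports success without reattaching.
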(event EventBeginPlay)

(event Collision|EventActorBeginOverlap
  (params (OtherActor :type Actor%20Object%20Reference)))

(event EventTick
  (params (DeltaSeconds :type Float%20%28single-precision%29)))

(fn ConstructionScript
  (Effects|Components|ParticleSystem|SetTemplate (Variables|Default|GetParticleSystem_0) (Variables|Default|GetHandParticle)))

(fn Attach
  (if (CallFunction|IsHidden)
    _
    (elif (CallFunction|IsOwnerinCombat)
      ;[0 0.272 1] If spell is not hidden and character is in combat, activate particle and attach to proper slot
      (Components|Activation|Activate (Variables|Default|GetParticleSystem_0) false)
      (bind _result (|CallParentFunction))
      (return _result)
      (else
        _)))
  ;[0 0.272 1] If spell is being hidden or character is not in combat, deactivate particle
  (Components|Activation|Deactivate (Variables|Default|GetParticleSystem_0))
  (return true))