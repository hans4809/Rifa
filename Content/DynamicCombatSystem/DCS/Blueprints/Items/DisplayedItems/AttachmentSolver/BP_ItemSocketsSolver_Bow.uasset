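; Socket solver for a displayed bow item, deciding which socket the bow attaches to.
; It returns the in-combat socket only when the item is visible and its owner is in combat, otherwise the out-of-combat socket.
; It also supplies the socket name used for spawning projectiles.
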(fn GetAttachSocketName
  (bind _displayeditem (Variables|Default|GetDisplayedItem))
  (if (Default|IsHidden _displayeditem)
    _
    (elif (Default|IsOwnerinCombat _displayeditem)
      (return (Variables|Default|GetInCombatSocketName))
      (else
        _)))
  (return (Variables|Default|GetOutCombatSocketName)))

(fn GetProjectileSpawnSocketName
  (return (Variables|Default|GetProjectileSpawnSocketName)))