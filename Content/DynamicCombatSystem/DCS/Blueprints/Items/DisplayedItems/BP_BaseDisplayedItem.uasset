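; Base actor for items displayed on a character's mesh in DCS, with hooks for equip, unequip and projectile spawn location.
; On BeginPlay it constructs an optional sockets solver object and can disable mesh collision.
; Attach snaps it to the socket that solver returns, and toggling hidden state re-runs Attach.
; Helpers query the owner's combat state and style, or switch all meshes to ragdoll physics.
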(event Custom|OnEquipped
  (bind _socketssolverclass (Variables|Default|GetSocketsSolverClass)
    (:then
      (bind _returnvalue (Game|ConstructObjectfromClass _socketssolverclass self))
      (Variables|Runtime|SetSocketsSolverObj _returnvalue))
    (:else)))

(event Custom|OnUnequipped)

(event EventBeginPlay
  (CallFunction|OnEquipped)
  (if (Variables|Default|GetAutoDisableCollisionOnComponents)
    (CallFunction|DisableCollisiononComponents)))

(event EventDestroyed
  (CallFunction|OnUnequipped))

(fn ConstructionScript)

(fn Attach
  (Transformation|AttachComponentToComponent (Variables|/Script/Engine.Character|GetMesh (.As캐릭터 (Utilities|Casting|CastToCharacter (Components|GetOwner)))) (CallFunction|GetAttachmentSocket) "SnapToTarget" "SnapToTarget" "KeepWorld" true)
  (return true))

(fn GetAttachmentSocket
  (bind _socketssolverobj (Variables|Runtime|GetSocketsSolverObj)
    (:then
      (bind _socketname (Default|GetAttachSocketName _socketssolverobj))
      (return _socketname))
    (:else
      (return "None"))))

(fn SimulatePhysics
  (bind _output_get (LocalVariables|SetL_PrimitiveComponents (Actor|GetComponentsByClass "/Script/Engine.MeshComponent")))
  (for _array_element _output_get
    (Collision|SetCollisionProfileName _array_element "Ragdoll" true :!class /Script/Engine.PrimitiveComponent)
    (Physics|SetSimulatePhysics _array_element true)))

(fn SetIsHidden
  (params (NewHidden :type Boolean))
  (if (!= NewHidden (Variables|Runtime|GetbIsHidden))
    (bind _output_get (Variables|Runtime|SetbIsHidden NewHidden))
    (Hidden|HiddenChanged _output_get)))

(fn IsHidden
  (return (Variables|Runtime|GetbIsHidden)))

(fn HiddenChanged
  (params (IsEnabled :type Boolean))
  (CallFunction|Attach))

(fn IsOwnerinCombat
  (return (Default|HasActivity (Actor|GetComponentbyClass (Components|GetOwner) "/Game/DynamicCombatSystem/DCS/Blueprints/Components/StateManager/BP_StateManagerComponent.BP_StateManagerComponent_C") "(GameplayTags=((TagName=\"Activity.IsInCombat\")))" "NewEnumerator0")))

(fn IsOwnersCombatStyle
  (params (CombatStyleTag :type Gameplay%20Tag%20Container%20Structure))
  (return (Default|IsCombatStyle (Actor|GetComponentbyClass (Components|GetOwner) "/Game/DynamicCombatSystem/DCS/Blueprints/Components/Combat/BP_CombatComponent.BP_CombatComponent_C") CombatStyleTag)))

(fn GetCollidingComponents
  (return (Actor|GetComponentsByClass "/Script/Engine.MeshComponent")))

(fn DisableCollisiononComponents
  (bind _output_get (LocalVariables|SetL_Components (Actor|GetComponentsByClass "/Script/Engine.MeshComponent")))
  (for _array_element _output_get
    (Collision|SetCollisionEnabled _array_element "NoCollision")))

(fn GetProjectileSpawnLocation
  ;[1 1 1] Should be overridden by items using projectiles ( bow / guns )
  (return "0, 0, 0"))