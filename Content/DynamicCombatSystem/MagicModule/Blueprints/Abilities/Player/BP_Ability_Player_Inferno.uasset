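; Player Inferno ability that casts an area damage effect on a targeted surface point within range.
; While held and not casting, Tick refreshes the target from a range- and slope-limited surface query and moves the spell indicator.
; Release starts casting with a montage and locks in the target, or hides the indicator if casting fails.
; The effect event spawns a damage sphere there with particle and sound, and applies the ability cost.
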(event Custom|SpawnParticle
  ;[0 0.272 1] Spawn Particle
  (Effects|SpawnEmitteratLocation (Variables|Ability|Custom|GetHitParticle) (CallFunction|GetEffectLocation)))

(event Custom|UpdateEffect
  ;[0 0.272 1] Update effect transform and it's indicator
  (bind _transform (CallFunction|GetSurfaceTransform (Variables|Ability|Custom|GetRange) (Variables|Ability|Custom|GetMaxSurfaceAngle) 2e+03))
  (Variables|Default|SetEffectTransform _transform)
  (CallFunction|UpdateIndicator (CallFunction|GetEffectLocation)))

(event Custom|PlaySound
  ;[0 0.272 1] Play Sound
  (Audio|PlaySoundatLocation (Variables|Ability|Custom|GetSound) (CallFunction|GetEffectLocation) "0, 0, 0" 1.0 1.0 0.0 0 0 0 0))

(event EventdReleased
  ;[0 0.272 1] On Ability released cast ability or hide spell indicator if not casting
  (bind _result (Default|StartCastingAbility (Variables|Default|GetAbilityComponent)))
  (if _result
    (CallFunction|PlayAbilityMontage (CallFunction|GetAbilityMontage) "None" -1.0)
    (CallFunction|UpdateEffect)
    (elif (not (Default|GetIsCasting (Variables|Default|GetAbilityComponent)))
      (CallFunction|HideIndicator))))

(event EventdPressed
  ;[0 0.272 1] On Ability pressed show spell indicator if not casting
  (if (not (Default|GetIsCasting (Variables|Default|GetAbilityComponent)))
    (CallFunction|UpdateEffect)
    (CallFunction|ShowIndicator (CallFunction|GetEffectLocation))))

(event EventTick
  (params (DeltaSeconds :type Float%20%28single-precision%29))
  (bind _abilitycomponent (Variables|Default|GetAbilityComponent))
  ;[0 0.272 1] Update effect transform only if ability is pressed but not already casting
  (if (and (Default|GetIsPressed _abilitycomponent) (not (Default|GetIsCasting _abilitycomponent)))
    (CallFunction|UpdateEffect)))

(event EventdSpawnEffect
  (bind _returnvalue (Components|GetOwner))
  ;[0 0.272 1] Effect
  (Game|SpawnActorfromClass "/Game/DynamicCombatSystem/DCS/Blueprints/Components/Ability/AbilityEffects/BP_AE_DamageSphere.BP_AE_DamageSphere_C" (Variables|Default|GetEffectTransform) "AlwaysSpawn" "OverrideRootScale" _returnvalue (Variables|Ability|Custom|GetRadius) (CallFunction|GetDamage 1.0) "None" (Game|GetInstigator _returnvalue))
  (CallFunction|SpawnParticle)
  (CallFunction|ApplyAbilityCost -1.0 1.0)
  (CallFunction|PlaySound))

(fn ConstructionScript
  (|CallParentFunction))

(fn UpdateEffectTransform
  (bind _location (CallFunction|GetEffectLocation))
  (bind _returnvalue (Components|GetOwner))
  (bind _returnvalue_2 (Transformation|GetActorLocation _returnvalue))
  (bind _z (Math|Vector|BreakVector _location))
  ;[0 0.272 1] Calculate Start/End trace location
  (LocalVariables|SetL_TraceStart _returnvalue_2)
  (LocalVariables|SetL_TraceEnd (+ _returnvalue_2 (* (Transformation|GetActorForwardVector (Pawn|GetController (Variables|/Script/Engine.Actor|GetInstigator _returnvalue))) (Variables|Ability|Custom|GetRange))))
  (bind _outhit (CallFunction|FindFloor (LocalVariables|GetL_TraceStart) (Variables|Ability|Custom|GetRange) 0.0))
  (if (.bBlockingHit (Collision|BreakHitResult _outhit))
    (LocalVariables|SetL_HitLocation (.Location (Collision|BreakHitResult _outhit)))
    (if (<= (Class|KismetMathLibrary|DegAcos (Math|Vector|DotProduct (.Normal (Collision|BreakHitResult _outhit)) "0, 0,1.000000")) (Math|Float|Absolute(Float) (Variables|Ability|Custom|GetMaxSurfaceAngle)))
      (LocalVariables|SetL_EffectLocation (LocalVariables|GetL_HitLocation))
      (else
        (LocalVariables|SetL_EffectLocation (Math|Vector|MakeVector (.X (Math|Vector|BreakVector (LocalVariables|GetL_HitLocation))) (.Y (Math|Vector|BreakVector (LocalVariables|GetL_HitLocation))) _z))))
    (else
      (LocalVariables|SetL_EffectLocation (Math|Vector|MakeVector (.X (Math|Vector|BreakVector (LocalVariables|GetL_TraceEnd))) (.Y (Math|Vector|BreakVector (LocalVariables|GetL_TraceEnd))) _z))))
  (return (Math|Transform|MakeTransform (LocalVariables|GetL_EffectLocation))))