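; BP_WaterTrigger is a gimmick volume that shows a waterfall widget while the player character is inside it and not swimming.
; On collision begin overlap it stores the BP_RifaCharacter_Final reference and, if not swimming, creates and adds WG_WaterFallWidget to the viewport.
; Tick removes the widget once that character swims or dies, and end overlap removes it as well.
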(event OnComponentBeginOverlap(CollisionComponent)
  (params (OverlappedComponent :type Primitive%20Component%20Object%20Reference) (OtherActor :type Actor%20Object%20Reference) (OtherComp :type Primitive%20Component%20Object%20Reference) (OtherBodyIndex :type Integer) (bFromSweep :type Boolean) (SweepResult :type Hit%20Result%20Structure%20%28by%20ref%29))
  (bind _asbp_rifa_character_final (Utilities|Casting|CastToBP_RifaCharacter_Final OtherActor))
  (bind _output_get (Variables|Default|SetCharacterReference _asbp_rifa_character_final))
  (if (not (Variables|/Script/Rifa.RifaCharacter|GetbIsSwimming _output_get))
    (bind _returnvalue (UserInterface|CreateWidget "/Game/BluePrint/UI/WG_WaterFallWidget.WG_WaterFallWidget_C"))
    (bind _output_get_2 (Variables|Default|SetWaterFallWidget _returnvalue))
    (UserInterface|Viewport|AddtoViewport _output_get_2 0)))

(event OnComponentEndOverlap(CollisionComponent)
  (params (OverlappedComponent :type Primitive%20Component%20Object%20Reference) (OtherActor :type Actor%20Object%20Reference) (OtherComp :type Primitive%20Component%20Object%20Reference) (OtherBodyIndex :type Integer))
  (bind _waterfallwidget (Variables|Default|GetWaterFallWidget))
  (Utilities|Casting|CastToBP_RifaCharacter_Final OtherActor)
  (if (Utilities|IsValid _waterfallwidget)
    (Widget|RemovefromParent _waterfallwidget)))

(event EventBeginPlay)

(event Collision|EventActorBeginOverlap
  (params (OtherActor :type Actor%20Object%20Reference)))

(event EventTick
  (params (DeltaSeconds :type Float%20%28single-precision%29))
  (bind _waterfallwidget (Variables|Default|GetWaterFallWidget))
  (bind _characterreference (Variables|Default|GetCharacterReference))
  (if (Utilities|IsValid _characterreference)
    (if (Variables|/Script/Rifa.RifaCharacter|GetbIsSwimming _characterreference)
      (if (Utilities|IsValid _waterfallwidget) :!label _label
        (Widget|RemovefromParent _waterfallwidget))
      (elif (Variables|/Script/Rifa.RifaCharacter|GetbIsDied _characterreference)
        (goto _label)))))

(fn ConstructionScript)